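; BP_Territory is a map territory actor that displays army count, owner and capital status.
; UpdateVisuals writes the army count to a text component, selects the plane's material by owner ID (only the first two options are assigned) and toggles the capital icon.
; UpdateFromData calls UpdateVisuals after setting the territory variables, but assigns blank defaults instead of reading NewData.
; Click, HUD and overlap logic is unconnected or disabled.
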(event `UpdateFromData`
  (params (NewData :type "/Game/Blueprints/Map/BP_Territory Object Reference"))
  (set `self.TerritoryID` 0)
  (set `self.TerritoryName` "")
  (set `self.OwnerPlayerID` 0)
  (set `self.IsCapital` false)
  (set `self.ArmyCount` (`KismetMathLibrary.Conv_Int64ToInt` 0))
  (`self.UpdateVisuals`))

(event `UpdateVisuals`
  (`TextRenderComponent.K2_SetText` (`self.ArmyTextRef`) (`KismetTextLibrary.Conv_IntToText` (`self.ArmyCount`)))
  (`PrimitiveComponent.SetMaterial` (`self.Visual Territory Plane`) 0 (select `int` (`self.OwnerPlayerID`) :`0` "/Engine/MapTemplates/Materials/BasicAsset01.BasicAsset01" :`1` "/Engine/MapTemplates/Materials/BasicAsset03.BasicAsset03" :`2` null :`3` null :`4` null :!type "MaterialInterface Object Reference"))
  (`SceneComponent.SetVisibility` (`self.CapitalIcon`) (`self.IsCapital`) false))

(fn `UserConstructionScript`)