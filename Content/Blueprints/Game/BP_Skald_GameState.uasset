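; Game state for Skald that holds territory and player data, with RepNotify variables whose handlers are empty.
; BeginPlay gathers all BP_Territory actors and matches them by ID against TerritoriesArray, writing entries back unchanged.
; SetTerritoryData overwrites an entry using TerritoryID as the array index.
; PreSizePlayersData rebuilds PlayersData on the authority with sequential player IDs, or clears it when the count is not positive.
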(event `self.ReceiveBeginPlay`
  (`/Engine/EditorBlueprintResources/ActorMacros.Switch Has Authority`
    (:`Authority`
      _)
    (:`Remote`
      _))
  (bind _outactors (`GameplayStatics.GetAllActorsOfClass` "/Game/Blueprints/Map/BP_Territory.BP_Territory_C"))
  (bind _output_get (set `self.AllTerritories` _outactors))
  (for (_array_element _array_index) _output_get
    (`KismetArrayLibrary.Array_Set` (`self.AllTerritories`) _array_index _array_element)
    (for (_array_element_2 _array_index_2) (`self.TerritoriesArray`)
      (if (== (`.TerritoryID_4_2A65E9294BFA08A0D60D27A9C8AC3699` (break `/Game/Blueprints/Structs/FS_Territory` _array_element_2)) (`/Game/Blueprints/Map/BP_Territory.TerritoryID` _array_element))
        (`KismetArrayLibrary.Array_Set` (`self.TerritoriesArray`) _array_index_2 _array_element_2)))))

(fn `OnRep_AllTerritories`)

(fn `OnRep_PlayersData`)

(fn `OnRep_SavePlayers`)

(fn `OnRep_TerritoriesArray`)

(fn `OnRep_TurnManagerRef`)

(fn `PreSizePlayersData`
  (params (InMaxPlayers :type Integer))
  (if (<= InMaxPlayers 0)
    (`KismetArrayLibrary.Array_Clear` (`self.PlayersData`))
    (else
      (`/Engine/EditorBlueprintResources/ActorMacros.Switch Has Authority`
        (:`Authority`
          (`KismetArrayLibrary.Array_Clear` (`self.PlayersData`))
          (for _index (range InMaxPlayers)
            (`KismetArrayLibrary.Array_Add` (`self.PlayersData`) (make `/Game/Blueprints/Structs/FS_PlayerData` _index))))))))

(fn `SetTerritoryData`
  (params (`New Data` :type "/Game/Blueprints/Structs/FS_Territory Structure"))
  (`KismetArrayLibrary.Array_Set` (`self.TerritoriesArray`) (`.TerritoryID_4_2A65E9294BFA08A0D60D27A9C8AC3699` (break `/Game/Blueprints/Structs/FS_Territory` `New Data`)) `New Data`))

(fn `UserConstructionScript`)