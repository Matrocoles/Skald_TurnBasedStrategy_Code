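; Player controller for Skald, a turn-based territory game, in which a left-click traces under the cursor and stores the hit territory.
; Retry events are written to cache the player ID and bind turn manager delegates, but nothing live starts them.
; BeginPlay, turn and phase handlers, and server action events are empty stubs.
; HUD creation, banner updates and other setup logic sit in disconnected nodes that never run.
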(event `self.ReceiveTick`
  (params (DeltaSeconds :type "Float (single-precision)"))
  (if (and (`self.bEnableClickEvents`) (`self.IsLocalController`))
    (if (and (`.bSuccess` (cast `/Game/Blueprints/Map/BP_Territory` (`.HitActor` (`GameplayStatics.BreakHitResult` (`self.GetHitResultUnderCursorByChannel` "TraceTypeQuery1"))) :!pure true)) false)
      _)))

(event `Key|LeftMouseButton`
  (params (Key :type "Key Structure"))
  ; Optional Highlight
)

(event `OnLocalTerritoryClicked`)

(event `OnTerritoryClicked`
  (params (TerritoryRef :type Name) (BP_Territory :type "/Game/Blueprints/Map/BP_Territory Object Reference")))

(event `Key|LeftMouseButton`
  (params (Key :type "Key Structure"))
  (bind (_asbp_territory _bsuccess) (cast `/Game/Blueprints/Map/BP_Territory` (`.HitActor` (`GameplayStatics.BreakHitResult` (`self.GetHitResultUnderCursorByChannel` "TraceTypeQuery1"))) :!pure true))
  ; Left Mouse Click
  (:`Pressed`
    (if _bsuccess
      (set `self.SelectedTerritoryRef ` _asbp_territory))))

(event `self.ReceiveBeginPlay`)

(event `Server_EndAttackPhase`)

(event `TryCachePlayerState`
  (bind _asbp_player_state_skald (cast `/Game/Blueprints/Game/BP_PlayerState_Skald` (`self.PlayerState`) :!pure true))
  (if (and (!= _asbp_player_state_skald null) (>= (`/Game/Blueprints/Game/BP_PlayerState_Skald.Skald_PlayerID` _asbp_player_state_skald) 0))
    (set `self.MySkaldPlayerID` (`/Game/Blueprints/Game/BP_PlayerState_Skald.Skald_PlayerID` _asbp_player_state_skald))
    (`KismetSystemLibrary.K2_ClearTimer` null "TryCachePlayerState")
    (else
      (`self.TryCachePlayerState`))))

(event `Server_RequestDigTreasure`)

(event `Server_EndMovementPhase`)

(event `RequestEngineeringAction`)

(event `TryBindTurnManager`
  (bind _tmref (`self.TMRef`))
  (if (== (`self.TMRef`) null)
    (bind _output_get (set `self.TMRef` (`/Game/Blueprints/Game/BP_Skald_GameState.TurnManagerRef` (`self.GS`))))
    (if (and (== _output_get null) (== (`self.bBoundTM`) false))
      (add `/Game/Blueprints/Game/BP_TurnManager.OnTurnStarted` _tmref (delegate `Handle_OnTurnStarted`))
      (add `/Game/Blueprints/Game/BP_TurnManager.OnPhaseChanged` _tmref (delegate `Handle_OnPhaseChanged`))
      (add `/Game/Blueprints/Game/BP_TurnManager.OnRequestHUDRefresh` _tmref (delegate `Handle_OnRequestHUDRefresh`))
      (set `self.bBoundTM` true)
      (`self.Handle_OnRequestHUDRefresh`)
      (else
        (`KismetSystemLibrary.K2_SetTimer` null "TryBindTurnManager" 0.25 true)))))

(event `Handle_OnTurnStarted`
  (params (PlayerID :type Integer) (TurnNumber :type Integer)))

(event `Handle_OnPhaseChanged`
  (params (PlayerID :type Integer) (NewPhase :type "/Game/Blueprints/Structs/E_TurnPhase Enum" :default "NewEnumerator0")))

(event `Handle_OnRequestHUDRefresh`)

(fn `UserConstructionScript`)