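; Server-side GameMode for Skald, a turn-based territory game with human and AI players.
; BeginPlay builds player data and starts a TryStartMatch timer, which gates InitializeMatch on MatchInitialized and human count.
; InitializeMatch fills GameState territories with random neutral armies, spawns BP_TurnManager and sets AI slots and turn order, while PostLogin assigns human slots.
; Capital assignment and save/load events are uncalled here, and loading restores no GameState data.
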(event `self.K2_PostLogin`
  (params (NewPlayer :type "PlayerController Object Reference"))
  (bind _asbp_skald_game_state (cast `/Game/Blueprints/Game/BP_Skald_GameState` (`GameplayStatics.GetGameState`) :!pure true))
  (bind _turnmanagerref (`/Game/Blueprints/Game/BP_Skald_GameState.TurnManagerRef` _asbp_skald_game_state))
  ; Post Login
  (bind _output_get (set `self.PS` (cast `/Game/Blueprints/Game/BP_PlayerState_Skald` (`Controller.PlayerState` NewPlayer) :!pure true)))
  (if (> (`KismetArrayLibrary.Array_Length` (`self.AvailableHumanSlots`)) 0)
    (bind _output_get_2 (set `self.Slot` (`|GetArrayItem` (`self.AvailableHumanSlots`))))
    (`KismetArrayLibrary.Array_Remove` (`self.AvailableHumanSlots`))
    (set `/Game/Blueprints/Game/BP_PlayerState_Skald.Skald_PlayerID` _output_get_2 _output_get)
    (bind _output_get_3 (set `/Game/Blueprints/Game/BP_PlayerState_Skald.DisplayName` (`KismetStringLibrary.Concat_StrStr` (`KismetStringLibrary.Conv_IntToString` _output_get_2) "Player") _output_get))
    (`KismetArrayLibrary.Array_Set` (`/Game/Blueprints/Game/BP_Skald_GameState.PlayersData` _asbp_skald_game_state) (`self.Slot`) (make `/Game/Blueprints/Structs/FS_PlayerData` :`PlayerID` (`self.Slot`) :`PlayerName` _output_get_3 :`IsHuman` true :`IsAlive` true) true)
    (if (`KismetSystemLibrary.IsValid` _turnmanagerref)
      (`/Game/Blueprints/Game/BP_TurnManager.OnRequestHUDRefresh` _turnmanagerref))))

(event `InitializeMatch`
  (params (NumPlayers :type "Integer (by ref)"))
  (bind _tempplayerorder (`self.TempPlayerOrder`))
  (bind _availablehumanslots (`self.AvailableHumanSlots`))
  (bind _gs (`self.GS`))
  (`/Engine/EditorBlueprintResources/ActorMacros.Switch Has Authority`
    (:`Authority`
      (if (not (`self.bUseSeed`))
        (set `self.MapSeed` (`KismetMathLibrary.RandomInteger` 1000)))
      (bind _output_get (set `self.GS` (cast `/Game/Blueprints/Game/BP_Skald_GameState` (`GameplayStatics.GetGameState`) :!pure true)))
      (set `/Game/Blueprints/Game/BP_Skald_GameState.TurnNumber` 1 _output_get)
      (bind _outactors (`GameplayStatics.GetAllActorsOfClass` "/Game/Blueprints/Map/BP_Territory.BP_Territory_C"))
      (bind _output_get_2 (set `self.AllTerritories` _outactors))
      (for (_array_element _array_index) _output_get_2
        (bind _output_get_3 (set `/Game/Blueprints/Map/BP_Territory.TerritoryID` _array_index _array_element))
        (set `self.TerrRef` _array_element)
        (`KismetArrayLibrary.Array_Clear` (`/Game/Blueprints/Game/BP_Skald_GameState.TerritoriesArray` (`self.GS`)))
        (for _ (range (`KismetArrayLibrary.Array_Length` (`self.AllTerritories`)))
          (set `self.InitialNeutralArmyMin` 150)
          (set `self.InitialNeutralArmyMax` 500)
          (`KismetArrayLibrary.Array_Add` (`/Game/Blueprints/Game/BP_Skald_GameState.TerritoriesArray` _gs) (make `/Game/Blueprints/Structs/FS_Territory` :`TerritoryID` (`/Game/Blueprints/Map/BP_Territory.TerritoryID` _array_element) :`TerritoryName` (`/Game/Blueprints/Map/BP_Territory.TerritoryName` _array_element) :`OwnerPlayerID` -1 :`ArmyCount` (`KismetMathLibrary.Conv_IntToInt64` (`KismetMathLibrary.RandomIntegerInRangeFromStream` (`self.RandomStream`) (`self.InitialNeutralArmyMin`) (`self.InitialNeutralArmyMax`))) :`ContinentID` (`/Game/Blueprints/Map/BP_Territory.ContinentID` _array_element)))
          (bind _returnvalue (`|SpawnActorFromClass` "/Game/Blueprints/Game/BP_TurnManager.BP_TurnManager_C" (`KismetMathLibrary.MakeTransform` (0.0 0.0 0.0)) "Undefined" "MultiplyWithRoot" null null))
          (bind _output_get_4 (set `/Game/Blueprints/Game/BP_Skald_GameState.TurnManagerRef` _returnvalue (`self.GS`)))
          (set `self.TurnManagerRef` _output_get_4)
          (`/Game/Blueprints/Game/BP_Skald_GameState.PreSizePlayersData` _gs (`self.MaxPlayers`))
          (if (> (`KismetArrayLibrary.Array_Length` _availablehumanslots) 0)
            (for (_array_element_2 _array_index_2) _availablehumanslots
              (`KismetArrayLibrary.Array_Set` (`/Game/Blueprints/Game/BP_Skald_GameState.PlayersData` (`self.GS`)) _array_index_2 (make `/Game/Blueprints/Structs/FS_PlayerData` :`PlayerID` _array_element_2 :`PlayerName` (`KismetStringLibrary.Concat_StrStr` (`KismetStringLibrary.Conv_IntToString` _array_element_2) "AI_") :`IsAI` true :`IsAlive` true))
              (set `/Game/Blueprints/Game/BP_TurnManager.PlayerOrder` (`self.TempPlayerOrder`) (`self.TurnManagerRef`))
              (for (_array_element_3 _array_index_3) (`/Game/Blueprints/Game/BP_Skald_GameState.PlayersData` (`self.GS`))
                (bind (_playerid _playername _isai _iseliminated) (break `/Game/Blueprints/Structs/FS_PlayerData` _array_element_3))
                (if (!= _iseliminated false)
                  (`KismetArrayLibrary.Array_Set` _tempplayerorder _array_index_3 _playerid)
                  (set `/Game/Blueprints/Game/BP_TurnManager.PlayerOrder` _tempplayerorder (`self.TurnManagerRef`))
                  (`KismetArrayLibrary.Array_Clear` (`self.AvailableHumanSlots`))
                  (`/Game/Blueprints/Game/BP_TurnManager.InitTurnManage` (`self.TurnManagerRef`) (`self.HumanCount`)))))))))
    (:`Remote`
      (`KismetSystemLibrary.PrintString` "Server Only"))))

(event `LoadGameLogic`
  (bind _asbp_skald_game_state (cast `/Game/Blueprints/Game/BP_Skald_GameState` (`GameplayStatics.GetGameState`) :!pure true))
  ; Load Game Event
  (bind _returnvalue (`GameplayStatics.LoadGameFromSlot` "SkaldSaveSlot"))
  (`/Engine/EditorBlueprintResources/StandardMacros.IsValid` _returnvalue
    (:`Is Valid`
      (set `self.TerritoryData` (`/Game/Blueprints/Game/BP_Skald_GameState.TerritoriesArray` _asbp_skald_game_state))
      (set `/Game/Blueprints/Game/BP_Skald_GameState.PlayersData` (`/Game/Blueprints/Game/BP_Skald_GameState.PlayersData` _asbp_skald_game_state) _asbp_skald_game_state)
      (bind _asbp_save_game (cast `/Game/Blueprints/Game/BP_SaveGame` _returnvalue :!pure true))
      (set `/Game/Blueprints/Game/BP_SaveGame.Sieges` (`/Game/Blueprints/Game/BP_SaveGame.Sieges` _asbp_save_game) _asbp_save_game)
      (set `/Game/Blueprints/Game/BP_SaveGame.TurnNumber` (`/Game/Blueprints/Game/BP_Skald_GameState.TurnNumber` _asbp_skald_game_state) _asbp_save_game)
      (set `/Game/Blueprints/Game/BP_SaveGame.CurrentPlayerIndex` (`/Game/Blueprints/Game/BP_SaveGame.CurrentPlayerIndex` _asbp_save_game) _asbp_save_game))))

(event `TryStartMatch`
  (if (== (`self.bMatchInitialized`) true)
    (bind _output_get (set `self.GS` (cast `/Game/Blueprints/Game/BP_Skald_GameState` (`GameplayStatics.GetGameState`) :!pure true)))
    (for _array_element (`/Game/Blueprints/Game/BP_Skald_GameState.PlayersData` _output_get)
      (bind _output_get_2 (set `self.HumanCount` (+ (`self.HumanCount`) 1)))
      (if (>= _output_get_2 (`self.MinHumansToStart`))
        (`KismetSystemLibrary.K2_ClearTimer` null "TryStartMatch")
        (set `self.bMatchInitialized` true)
        (`self.InitializeMatch` (`self.HumanCount`))
        (`KismetSystemLibrary.PrintString` "InitializeMatch called (Humans= X)")))
    (else
      (`KismetSystemLibrary.K2_ClearTimer` null "TryStartMatch")
      (`self.ReturnToMainMenuHost`))))

(event `SaveGameLogic`
  (bind _asbp_skald_game_state (cast `/Game/Blueprints/Game/BP_Skald_GameState` (`GameplayStatics.GetGameState`) :!pure true))
  ; Save Game Event
  (bind _returnvalue (`GameplayStatics.CreateSaveGameObject` "/Game/Blueprints/Game/BP_SaveGame.BP_SaveGame_C"))
  (bind _output_get (set `/Game/Blueprints/Game/BP_SaveGame.SaveName` "SkaldSaveSlot" _returnvalue))
  (set `/Game/Blueprints/Game/BP_SaveGame.SaveDate` (`KismetTextLibrary.Conv_TextToString` (`KismetTextLibrary.AsTimeZoneDate_DateTime` (`KismetMathLibrary.Now`))) _returnvalue)
  (set `/Game/Blueprints/Game/BP_SaveGame.TurnNumber` (`self.CurrentTurnIndex`) _returnvalue)
  (set `/Game/Blueprints/Game/BP_SaveGame.CurrentPlayerIndex` (`/Game/Blueprints/Game/BP_SaveGame.CurrentPlayerIndex` _returnvalue) _returnvalue)
  (set `/Game/Blueprints/Game/BP_SaveGame.Territories` (`/Game/Blueprints/Game/BP_Skald_GameState.TerritoriesArray` _asbp_skald_game_state) _returnvalue)
  (set `/Game/Blueprints/Game/BP_Skald_GameState.PlayersData` (`/Game/Blueprints/Game/BP_Skald_GameState.PlayersData` _asbp_skald_game_state) _asbp_skald_game_state)
  (set `/Game/Blueprints/Game/BP_SaveGame.Players` (`/Game/Blueprints/Game/BP_Skald_GameState.SavePlayers` _asbp_skald_game_state) _returnvalue)
  (set `/Game/Blueprints/Game/BP_SaveGame.RandomSeed` (`self.MapSeed`) _returnvalue)
  (`GameplayStatics.SaveGameToSlot` _returnvalue _output_get))

(event `self.ReceiveBeginPlay`
  (`/Engine/EditorBlueprintResources/ActorMacros.Switch Has Authority`
    (:`Authority`
      (`KismetSystemLibrary.PrintString` "GameMode BeginPlay (server)")
      ; Begin Play
      (if (`self.bAutoStartOnBeginPlay`)
        (`self.BuildPlayersData`)
        (`/Game/Blueprints/Game/BP_Skald_GameState.PreSizePlayersData` (cast `/Game/Blueprints/Game/BP_Skald_GameState` (`GameplayStatics.GetGameState`) :!pure true) (`self.MaxPlayers`))
        (`KismetSystemLibrary.K2_SetTimer` null "TryStartMatch" 1.0 true)
        (else
          (`self.ReturnToMainMenuHost`))))))

(event `AssignInitialCapitals`
  (bind _randomstream (`self.RandomStream`))
  ; Assing Capitals
  (bind _output_get (set `self.TerritoriesPool` (`self.AllTerritories`)))
  (`KismetArrayLibrary.Array_ShuffleFromStream` _output_get _randomstream)
  (for _index (range (- (`KismetArrayLibrary.Array_Length` _output_get) 1) (+ (`KismetMathLibrary.RandomIntegerInRangeFromStream` _randomstream 0 42) 1))
    (`KismetArrayLibrary.Array_Swap` _output_get _index (`KismetMathLibrary.RandomIntegerInRange` _index 43))
    (bind _output (`|GetArrayItem` _output_get _index))
    (bind _output_get_2 (set `/Game/Blueprints/Map/BP_Territory.IsCapital` true _output))
    (bind _output_get_3 (set `/Game/Blueprints/Map/BP_Territory.OwnerPlayerID` (`/Game/Blueprints/Map/BP_Territory.OwnerPlayerID` _output) _output))
    (`KismetArrayLibrary.Array_Set` (`/Game/Blueprints/Game/BP_Skald_GameState.TerritoriesArray` (`self.GS`)) 0 (make `/Game/Blueprints/Structs/FS_Territory` (`/Game/Blueprints/Map/BP_Territory.TerritoryID` _output) (`/Game/Blueprints/Map/BP_Territory.TerritoryName` _output) _output_get_3 _output_get_2 _output_get_3)))
  (`KismetSystemLibrary.PrintString` "Capital assigned: \" + TerritoryName + \" → Player \" + PlayerID"))

(event `BuildPlayersData`
  (bind _asbp_skald_game_state (cast `/Game/Blueprints/Game/BP_Skald_GameState` (`GameplayStatics.GetGameState`) :!pure true))
  (bind _playersdata (`/Game/Blueprints/Game/BP_Skald_GameState.PlayersData` (`self.GS`)))
  (bind _playersdata_2 (`/Game/Blueprints/Game/BP_Skald_GameState.PlayersData` (`self.GS`)))
  (bind _returnvalue (`KismetArrayLibrary.Array_Length` _playersdata))
  (bind _output_get (set `self.GS` _asbp_skald_game_state))
  (`KismetArrayLibrary.Array_Clear` (`/Game/Blueprints/Game/BP_Skald_GameState.PlayersData` _asbp_skald_game_state))
  (for (_array_element _array_index) (`GameStateBase.PlayerArray` _output_get)
    (`KismetArrayLibrary.Array_Add` _playersdata_2 (make `/Game/Blueprints/Structs/FS_PlayerData` :`PlayerID` _array_index :`PlayerName` (`PlayerState.GetPlayerName` _array_element) :`IsHuman` true :`IsAlive` true))
    (bind _output_get_2 (set `self.Remainingslots` (- (`self.MaxPlayers`) (`KismetArrayLibrary.Array_Length` _playersdata_2))))
    (for _index (range _output_get_2)
      (`KismetArrayLibrary.Array_Set` _playersdata _returnvalue (make `/Game/Blueprints/Structs/FS_PlayerData` :`PlayerID` _returnvalue :`PlayerName` (`KismetStringLibrary.Concat_StrStr` "Ai_" (`KismetStringLibrary.Conv_IntToString` _index)) :`IsAI` true :`IsAlive` true)))))

(fn `UserConstructionScript`)