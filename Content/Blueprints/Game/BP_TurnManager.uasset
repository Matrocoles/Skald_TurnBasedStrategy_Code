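; BP_TurnManager is a mostly unwired turn manager for a networked turn-based game with player order, turn numbers and phases including revolt and reinforcement.
; Its only live logic forwards OnTurnStarted_Event to OnTurnStartedEvent.
; Authority-gated logic for setup, player order and turn start is disconnected and never runs.
; BeginPlayerTurn, the phase functions and all OnRep handlers are empty stubs.
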(event `BeginPlayerTurn`)

(event `OnTurnStarted_Event`
  (params (PlayerID :type Integer) (TurnNumber :type Integer))
  (`self.OnTurnStarted_Event` PlayerID TurnNumber))

(fn `BeginPhase_Reinforcement`
  (params (CurrentplayerID :type Integer)))

(fn `InitTurnManage`
  (params (NumPlayers :type Integer)))

(fn `OnRep_bIsTurnActive`)

(fn `OnRep_CurrentPhase`)

(fn `OnRep_CurrentTurnIndex`)

(fn `OnRep_PlayerOrder`)

(fn `OnRep_TurnNumber`)

(fn `OnRep_TurnTimeLimit`)

(fn `OnRep_TurnTimerHandle`)

(fn `ResolveRevoltPhase`
  (params (PlayerID :type Integer)))

(fn `SetPlayerOrder`
  (params (InOrder :type "Array of Integer")))

(fn `UserConstructionScript`)